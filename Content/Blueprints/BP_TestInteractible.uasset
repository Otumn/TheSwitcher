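; BP_TestInteractible is a test interactable actor that shows hover state by recoloring its Sphere.
; On BeginPlay it binds to the hovered and unhovered events of its BPInteractableComponent.
; Hovering sets the "Color" vector parameter on the sphere's materials to red, and unhovering sets it to white.
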(event `self.ReceiveBeginPlay`
  (bind _bp_interactablecomponent (`self.BP_interactableComponent`))
  (add `/Game/Blueprints/BP_interactableComponent.HoveredEvent` _bp_interactablecomponent (`|CreateDelegate` :!event `Hovered`))
  (add `/Game/Blueprints/BP_interactableComponent.UnHoveredEvent` _bp_interactablecomponent (`|CreateDelegate` :!event `Unhovered`)))

(event `Hovered`
  (`MeshComponent.SetVectorParameterValueOnMaterials` (`self.Sphere`) "Color" (1.0 0.0 0.0)))

(event `Unhovered`
  (`MeshComponent.SetVectorParameterValueOnMaterials` (`self.Sphere`) "Color" (1.0 1.0 1.0)))

(fn `UserConstructionScript`)