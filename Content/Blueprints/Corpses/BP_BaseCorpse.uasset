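; BP_BaseCorpse is a base corpse actor with a targeting indicator that can be shown or hidden.
; ActivateTargetting and DeactivateTargetting toggle the TargetWidget's visibility, and both enable actor tick, so deactivation does not stop it.
; Each tick, HUDFacingPlayer billboards the widget by rotating it toward the first player's camera manager with a look-at rotation.
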(event `self.ReceiveTick`
  (params (DeltaSeconds :type "Float (single-precision)"))
  (`self.HUDFacingPlayer`))

(event `ActivateTargetting`
  (`SceneComponent.SetVisibility` (`self.TargetWidget`) true false)
  (`self.SetActorTickEnabled` true))

(event `DeactivateTargetting`
  (`SceneComponent.SetVisibility` (`self.TargetWidget`) false false)
  (`self.SetActorTickEnabled` true))

(fn `HUDFacingPlayer`
  (`SceneComponent.K2_SetWorldRotation` (`self.TargetWidget`) (`KismetMathLibrary.FindLookAtRotation` (`SceneComponent.K2_GetComponentLocation` (`self.TargetWidget`)) (`self.K2_GetActorLocation` (`GameplayStatics.GetPlayerCameraManager` 0))) false false))

(fn `UserConstructionScript`)