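; Health pickup collectible that heals the player when interacted with.
; On Interacted, it calls HealPlayer on the official player pawn with StatAmount, then destroys itself.
; The construction script pushes its Color and EmissivePower into the mesh materials and tints the particle effect to match.
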(event `self.Interacted`
  (`/Game/Blueprints/Player/BP_BasePlayerPawn.HealPlayer` (`/Game/Blueprints/BP_CommonLibrary.GetPlayerOfficialPawn`) (`self.StatAmount`))
  (`self.K2_DestroyActor`))

(fn `UserConstructionScript`
  (bind _returnvalue (`KismetMathLibrary.Conv_LinearColorToVector` (`self.Color`)))
  (`parent.UserConstructionScript`)
  (`MeshComponent.SetScalarParameterValueOnMaterials` (`self.Mesh`) "Emissive" (`self.EmissivePower`))
  (`MeshComponent.SetVectorParameterValueOnMaterials` (`self.Mesh`) "Color" _returnvalue)
  (`FXSystemComponent.SetVectorParameter` (`self.Particles`) "ParticleColor" _returnvalue))