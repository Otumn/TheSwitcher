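; BP_BaseCollectible is a base collectible actor that shows a widget while hovered and turns it toward the player.
; On BeginPlay it binds hover, unhover and interact handlers to its BPInteractableComponent.
; Hover and unhover toggle the widget's visibility, though both enable actor tick, which runs SceneComponentFacePlayer on the widget.
; The Interacted event is empty, so this class defines no pickup behavior.
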(event `self.ReceiveBeginPlay`
  (`self.SetupEvents`))

(event `self.ReceiveTick`
  (params (DeltaSeconds :type "Float (single-precision)"))
  (`/Game/Blueprints/BP_CommonLibrary.SceneComponentFacePlayer` (`self.Widget`)))

(event `Hovered`
  (`SceneComponent.SetVisibility` (`self.Widget`) true false)
  (`self.SetActorTickEnabled` true))

(event `Unhovered`
  (`SceneComponent.SetVisibility` (`self.Widget`) false false)
  (`self.SetActorTickEnabled` true))

(event `Interacted`)

(fn `SetupEvents`
  (add `/Game/Blueprints/BP_interactableComponent.HoveredEvent` (`self.BP_interactableComponent`) (`|CreateDelegate` :!event `Hovered`))
  (add `/Game/Blueprints/BP_interactableComponent.UnHoveredEvent` (`self.BP_interactableComponent`) (`|CreateDelegate` :!event `Unhovered`))
  (add `/Game/Blueprints/BP_interactableComponent.InteractedEvent` (`self.BP_interactableComponent`) (`|CreateDelegate` :!event `Interacted`)))

(fn `UserConstructionScript`)