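; BP_CommonLibrary is a library of shared helper functions for reaching core game objects and orienting components toward the player.
; GetGameMaster and GetPlayerOfficialPawn return the game instance as BP_GameInstance and player 0's pawn as BP_BasePlayerPawn.
; SceneComponentFacePlayer sets a component's world rotation with a look-at toward player 0's camera manager, so it faces the view rather than the pawn.
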(fn `GetGameMaster`
  (returns (GameMaster :type "/Game/Blueprints/BP_GameInstance Object Reference"))
  (return (cast `/Game/Blueprints/BP_GameInstance` (`GameplayStatics.GetGameInstance` null) :!pure true)))

(fn `GetPlayerOfficialPawn`
  (returns (PlayerPawn :type "/Game/Blueprints/Player/BP_BasePlayerPawn Object Reference"))
  (return (cast `/Game/Blueprints/Player/BP_BasePlayerPawn` (`GameplayStatics.GetPlayerPawn` null) :!pure true)))

(fn `SceneComponentFacePlayer`
  (params (Scene :type "SceneComponent Object Reference"))
  (`SceneComponent.K2_SetWorldRotation` Scene (`KismetMathLibrary.FindLookAtRotation` (`SceneComponent.K2_GetComponentLocation` Scene) (`Actor.K2_GetActorLocation` (`GameplayStatics.GetPlayerCameraManager` null))) false false))